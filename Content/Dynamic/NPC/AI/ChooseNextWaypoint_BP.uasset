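; Behavior tree task that picks the next patrol waypoint for an AI-controlled NPC.
; It casts the controlled pawn to read its patrol points, then writes the point at the current blackboard index into the waypoint key.
; It then increments the index with a modulo wrap, so the route loops, and finishes with success.
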(event `self.ReceiveExecuteAI`
  (params (OwnerController :type "AIController Object Reference") (ControlledPawn :type "Pawn Object Reference"))
  (`self.GetPatrolPoints` ControlledPawn)
  (bind _index (`self.SetNextWayPoint`))
  (`self.CycleIndex` _index)
  (`self.FinishExecute` true))

(fn `CycleIndex`
  (params (Index :type Integer))
  (`BTFunctionLibrary.SetBlackboardValueAsInt` (`self.Index`) (mod (+ Index 1) (`KismetArrayLibrary.Array_Length` (`self.PatrolPoints`)))))

(fn `GetPatrolPoints`
  (params (Object :type "Object Object Reference"))
  (cast `` Object)
  (set `self.PatrolPoints` (`self.Patrol Points`)))

(fn `SetNextWayPoint`
  (returns (Index :type Integer))
  (bind _returnvalue (`BTFunctionLibrary.GetBlackboardValueAsInt` (`self.Index`)))
  (`BTFunctionLibrary.SetBlackboardValueAsObject` (`self.WayPoint`) (`KismetArrayLibrary.Array_Get` (`self.PatrolPoints`) _returnvalue))
  (return _returnvalue))