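; NPC AI controller that runs a guard behaviour tree on a patrol blackboard.
; AI Perception updates set the blackboard enemy key when an actor without the "Robot" tag is sensed, and clear it when sensing fails, printing each change.
; Helper functions, not called in this graph, seed the first patrol waypoint behind an unresolved cast and print sense debug info.
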(event `self.ReceiveBeginPlay`
  ;[1 1 1] Setting up initial behaviour tree to use and initialization
  (bind _blackboardcomponent (`self.UseBlackboard` "/Game/Dynamic/NPC/AI/PatrolData.PatrolData"))
  (`self.RunBehaviorTree` "/Game/Dynamic/NPC/AI/GuardBehaviour.GuardBehaviour")
  (set `self.BlackboardComponent` _blackboardcomponent))

(event `self.AIPerception.OnTargetPerceptionUpdated`
  (params (Actor :type "Actor Object Reference") (Stimulus :type "AIStimulus Structure"))
  (bind _blackboardcomponent (`self.BlackboardComponent`))
  (bind _enemykey (`self.EnemyKey`))
  ;[1 1 1] When AI sees or hears something - Set/Unset Player blackboard var
  (if (`self.ActorHasTag` Actor "Robot")
    _
    (elif (`.bSuccessfullySensed` (break `AIStimulus` Stimulus))
      (`BlackboardComponent.SetValueAsObject` _blackboardcomponent _enemykey Actor)
      (`KismetSystemLibrary.PrintString` "Player is SET")
      (else
        (`BlackboardComponent.ClearValue` _blackboardcomponent _enemykey)
        (`KismetSystemLibrary.PrintString` "Player is UNSET")))))

(fn `Find Patrol Route`
  (params (Blackboard :type "BlackboardComponent Object Reference"))
  (cast `` _)
  (`BlackboardComponent.SetValueAsObject` Blackboard "WayPoint" (`KismetArrayLibrary.Array_Get` (`self.Patrol Points`))))

(fn `SensoryDebugOutput`
  (params (`Sensed Actor` :type "Object Object Reference") (Stimulus :type "AIStimulus Structure (by ref)"))
  (bind _returnvalue (`AIPerceptionSystem.GetSenseClassForStimulus` Stimulus))
  (`KismetSystemLibrary.PrintString` (`KismetStringLibrary.Concat_StrStr` "Guard " (`KismetSystemLibrary.GetDisplayName` (`self.K2_GetPawn`)) " " (`KismetSystemLibrary.GetClassDisplayName` _returnvalue) " " (`KismetSystemLibrary.GetDisplayName` `Sensed Actor`))))

(fn `UserConstructionScript`)